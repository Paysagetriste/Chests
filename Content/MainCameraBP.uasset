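; MainCameraBP is a camera actor that centers itself above an area spanned by a first and last square, likely a grid board.
; The SetCameraLocation event receives both square locations, waits briefly, then moves the actor to their XY midpoint at a fixed height.
; It changes only location, with no rotation or zoom logic, and has no active BeginPlay, Tick or construction logic.
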(event `Set Camera Location`
  (params (`First square Location` :type "Vector Structure") (`Last square Location` :type "Vector Structure"))
  (bind _x (.x `First square Location`))
  (bind _y (.y `First square Location`))
  (`KismetSystemLibrary.Delay` 0.2)
  (`self.K2_SetActorLocation` (`KismetMathLibrary.MakeVector` (+ (/ (- (.x `Last square Location`) _x) 2.0) _x) (+ (/ (- (.y `Last square Location`) _y) 2.0) _y) 1500.0)))

(fn `UserConstructionScript`)